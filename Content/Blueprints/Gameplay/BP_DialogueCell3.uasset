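; BP_DialogueCell3 is a dialogue trigger actor that feeds lines from its dialogue component to the interacting pawn's dialogue widget.
; Activate reads the current row's speaker and long dialogue text, pushes them to the widget, and starts the dialogue with the pawn's Dice.
; Update advances to the next row and refreshes the widget, or exits and resets the row to zero once the dialogue is finished.
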(event EventBeginPlay
  (|CallParentFunction) ; This node is disabled and will not be called.\nDrag off pins to build functionality.
)

(event Collision|EventActorBeginOverlap
  (params (OtherActor :type Actor%20Object%20Reference))
  (|CallParentFunction OtherActor) ; This node is disabled and will not be called.\nDrag off pins to build functionality.
)

(event EventTick
  (params (DeltaSeconds :type Float%20%28single-precision%29))
  (|CallParentFunction DeltaSeconds) ; This node is disabled and will not be called.\nDrag off pins to build functionality.
)

(event EventActivate
  (params (Pawn :type BP%20Pawn%20Object%20Reference))
  (bind _widget (Variables|/Game/Blueprints/Gameplay/BP_Pawn.BP_Pawn_C|GetWidget Pawn))
  (bind _bpc_dialoguecomponent (Variables|Default|GetBPC_DialogueComponent))
  (Default|GetCurrentDialogueRowData _bpc_dialoguecomponent)
  (bind _charactername (Default|GetCharacterfromRow _bpc_dialoguecomponent))
  (bind _dialoguelong (Default|GetDialogueLongfromCurrentRow _bpc_dialoguecomponent))
  (Default|UptadeDialogue _widget _charactername _dialoguelong)
  (Default|StartDialogue _widget (Variables|/Game/Blueprints/Gameplay/BP_Pawn.BP_Pawn_C|GetDice Pawn)))

(event EventUpdate
  (params (Pawn :type BP%20Pawn%20Object%20Reference))
  (bind _bpc_dialoguecomponent (Variables|Default|GetBPC_DialogueComponent))
  (bind _widget (Variables|/Game/Blueprints/Gameplay/BP_Pawn.BP_Pawn_C|GetWidget Pawn))
  (bind _isdialoguefinished (Default|IsDialogueFinished (Variables|Default|GetBPC_DialogueComponent)))
  (if _isdialoguefinished
    (Default|ExitDialogue _widget)
    (Variables|/Game/Global/BPC_DialogueComponent.BPC_DialogueComponent_C|SetCurrentRowNumber (Variables|Default|GetBPC_DialogueComponent) 0)
    (else
      (Default|ReadtheNextRow (Variables|Default|GetBPC_DialogueComponent))
      (Default|GetCurrentDialogueRowData _bpc_dialoguecomponent)
      (bind _charactername (Default|GetCharacterfromRow _bpc_dialoguecomponent))
      (bind _dialoguelong (Default|GetDialogueLongfromCurrentRow _bpc_dialoguecomponent))
      (Default|UptadeDialogue _widget _charactername _dialoguelong))))

(fn ConstructionScript
  (|CallParentFunction))