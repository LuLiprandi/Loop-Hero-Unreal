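; BP_Pawn is the player's token on a cell-based board, with its cell number and Fear stored in BP_LoopGameInstance.
; On BeginPlay it snaps to the saved cell, creates the dialogue and fear gauge widgets, and gets possessed by the first player controller.
; TryMoving asks the Board for the destination, saves it, teleports the pawn there and activates the cell.
; UpdateCell refreshes the current cell's message.
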(event EventBeginPlay
  (bind _asbp_loop_game_instance (Utilities|Casting|CastToBP_LoopGameInstance (Game|GetGameInstance)))
  (Variables|Default|SetAs%20BP%20Loop%20Game%20Instance _asbp_loop_game_instance)
  (CallFunction|MovetoCell)
  (bind _returnvalue (UserInterface|CreateWidget "/Game/Global/WBP_DialogueUI.WBP_DialogueUI_C"))
  (bind _output_get (Variables|Default|SetWidget _returnvalue))
  (Variables|/Game/Global/WBP_DialogueUI.WBP_DialogueUI_C|SetPawn _output_get self)
  (UserInterface|Viewport|AddtoViewport _output_get 0)
  (Pawn|Possess (Game|GetPlayerController 0) self)
  (bind _returnvalue_2 (UserInterface|CreateWidget "/Game/Widget/WBP_Jauge.WBP_Jauge_C"))
  (bind _output_get_2 (Variables|Default|SetJaugeBar _returnvalue_2))
  (Progress|SetPercent (Variables|/Game/Widget/WBP_Jauge.WBP_Jauge_C|GetJaugeBar _output_get_2) (/ (Math|Conversions|ToFloat(Integer) (Variables|/Game/Global/BP_LoopGameInstance.BP_LoopGameInstance_C|GetFear (Variables|Default|GetAs%20BP%20Loop%20Game%20Instance))) 1e+02))
  (UserInterface|Viewport|AddtoViewport _output_get_2 0))

(event Collision|EventActorBeginOverlap
  (params (OtherActor :type Actor%20Object%20Reference)))

(event EventTick
  (params (DeltaSeconds :type Float%20%28single-precision%29)))

(fn ConstructionScript)

(fn MovetoCell
  (bind _cell (Default|GetCellbyNumber (Variables|Default|GetBoard) (Variables|/Game/Global/BP_LoopGameInstance.BP_LoopGameInstance_C|GetCellNumber (Variables|Default|GetAs%20BP%20Loop%20Game%20Instance))))
  (Transformation|SetActorLocation (.location (Transformation|GetActorTransform _cell)) false false)
  (Transformation|SetActorRotation (.rotation (Transformation|GetActorTransform _cell))))

(fn TryMoving
  (params (Value :type Integer))
  (bind _as_bp_loop_game_instance (Variables|Default|GetAs%20BP%20Loop%20Game%20Instance))
  (bind _cell (Default|GetNextCelltoMove (Variables|Default|GetBoard) (+ Value (Variables|/Game/Global/BP_LoopGameInstance.BP_LoopGameInstance_C|GetCellNumber _as_bp_loop_game_instance)) (Variables|Default|GetAs%20BP%20Loop%20Game%20Instance)))
  (Variables|/Game/Global/BP_LoopGameInstance.BP_LoopGameInstance_C|SetCellNumber _as_bp_loop_game_instance _cell)
  (CallFunction|MovetoCell)
  (CallFunction|ActivateCell))

(fn ActivateCell
  (bind _cell (Default|GetCellbyNumber (Variables|Default|GetBoard) (Variables|/Game/Global/BP_LoopGameInstance.BP_LoopGameInstance_C|GetCellNumber (Variables|Default|GetAs%20BP%20Loop%20Game%20Instance))))
  (Default|Activate _cell self))

(fn UpdateCell
  (bind _cell (Default|GetCellbyNumber (Variables|Default|GetBoard) (Variables|/Game/Global/BP_LoopGameInstance.BP_LoopGameInstance_C|GetCellNumber (Variables|Default|GetAs%20BP%20Loop%20Game%20Instance))))
  (Class|BPIActivate|Update(Message) _cell self))