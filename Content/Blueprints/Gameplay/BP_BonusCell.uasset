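; Bonus cell that lowers the player's fear when activated with a pawn.
; Activate subtracts a fixed amount from Fear on the loop game instance referenced by the pawn, clamped to the gauge range.
; It then pushes the normalized value directly to the pawn's JaugeBar progress bar.
; BeginPlay, overlap and Tick are unused, so Activate must be invoked from outside this graph.
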(event EventBeginPlay
  (|CallParentFunction) ; This node is disabled and will not be called.\nDrag off pins to build functionality.
)

(event Collision|EventActorBeginOverlap
  (params (OtherActor :type Actor%20Object%20Reference))
  (|CallParentFunction OtherActor) ; This node is disabled and will not be called.\nDrag off pins to build functionality.
)

(event EventTick
  (params (DeltaSeconds :type Float%20%28single-precision%29))
  (|CallParentFunction DeltaSeconds) ; This node is disabled and will not be called.\nDrag off pins to build functionality.
)

(event EventActivate
  (params (Pawn :type BP%20Pawn%20Object%20Reference))
  (bind _as_bp_loop_game_instance (Variables|/Game/Blueprints/Gameplay/BP_Pawn.BP_Pawn_C|GetAs%20BP%20Loop%20Game%20Instance Pawn))
  (bind _output_get (Variables|/Game/Global/BP_LoopGameInstance.BP_LoopGameInstance_C|SetFear _as_bp_loop_game_instance (Math|Integer|Clamp(Integer) (- (Variables|/Game/Global/BP_LoopGameInstance.BP_LoopGameInstance_C|GetFear _as_bp_loop_game_instance) 5) 0 100)))
  (Progress|SetPercent (Variables|/Game/Widget/WBP_Jauge.WBP_Jauge_C|GetJaugeBar (Variables|/Game/Blueprints/Gameplay/BP_Pawn.BP_Pawn_C|GetJaugeBar Pawn)) (/ (Math|Conversions|ToFloat(Integer) _output_get) 1e+02)))

(fn ConstructionScript
  (|CallParentFunction))