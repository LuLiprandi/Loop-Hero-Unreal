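; BP_CellsEnd is the end point that finishes the game when activated by a player holding the key.
; Its Activate event checks HaveKey on the loop game instance referenced through the passed Pawn.
; If the key is held, it shows the WBP_Victory widget, waits briefly, then quits the game.
; Without the key, activation does nothing.
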(event EventBeginPlay
  (|CallParentFunction) ; This node is disabled and will not be called.\nDrag off pins to build functionality.
)

(event Collision|EventActorBeginOverlap
  (params (OtherActor :type Actor%20Object%20Reference))
  (|CallParentFunction OtherActor) ; This node is disabled and will not be called.\nDrag off pins to build functionality.
)

(event EventTick
  (params (DeltaSeconds :type Float%20%28single-precision%29))
  (|CallParentFunction DeltaSeconds) ; This node is disabled and will not be called.\nDrag off pins to build functionality.
)

(event EventActivate
  (params (Pawn :type BP%20Pawn%20Object%20Reference))
  (if (Variables|/Game/Global/BP_LoopGameInstance.BP_LoopGameInstance_C|GetHaveKey (Variables|/Game/Blueprints/Gameplay/BP_Pawn.BP_Pawn_C|GetAs%20BP%20Loop%20Game%20Instance Pawn))
    (bind _returnvalue (UserInterface|CreateWidget "/Game/Widget/WBP_Victory.WBP_Victory_C"))
    (UserInterface|Viewport|AddtoViewport _returnvalue 0)
    (Utilities|FlowControl|Delay 3.0)
    (Game|QuitGame 0 "Quit" false)))

(fn ConstructionScript
  (|CallParentFunction))