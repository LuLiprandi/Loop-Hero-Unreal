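; BP_Dice is the dice actor that produces random rolls to move a pawn.
; On BeginPlay it shows the mouse cursor, creates the WBP_DiceRool widget, passes itself to it as Dice and adds it to the viewport.
; RollTheDice picks a random integer from one to six and passes it to TryMoving on its referenced Pawn.
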(event EventBeginPlay
  (Variables|/Script/Engine.PlayerController|SetbShowMouseCursor (Game|GetPlayerController 0) true)
  (bind _returnvalue (UserInterface|CreateWidget "/Game/Blueprints/HUD/Widget/WBP_DiceRool.WBP_DiceRool_C"))
  (bind _output_get (Variables|Default|SetDiceRoll _returnvalue))
  (Variables|/Game/Blueprints/HUD/Widget/WBP_DiceRool.WBP_DiceRool_C|SetDice _output_get self)
  (UserInterface|Viewport|AddtoViewport _output_get 0))

(event Collision|EventActorBeginOverlap
  (params (OtherActor :type Actor%20Object%20Reference)))

(event EventTick
  (params (DeltaSeconds :type Float%20%28single-precision%29)))

(fn ConstructionScript)

(fn RolltheDice
  (LocalVariables|SetValue (Math|Random|RandomIntegerinRange 1 6))
  (Default|TryMoving (Variables|Default|GetPawn) (LocalVariables|GetValue)))