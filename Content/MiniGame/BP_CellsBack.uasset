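; BP_CellsBack is a minigame exit trigger that completes the level once the player has collected all plushes.
; On any Box overlap, it reads the BP_FirstPerson player character and compares PlushCollected to TotalPlush, without checking which actor overlapped.
; When the count is met, it shows the WBP_Victory widget, waits briefly, then opens the MLoopHero level.
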(event OnComponentBeginOverlap(Box)
  (params (OverlappedComponent :type Primitive%20Component%20Object%20Reference) (OtherActor :type Actor%20Object%20Reference) (OtherComp :type Primitive%20Component%20Object%20Reference) (OtherBodyIndex :type Integer) (bFromSweep :type Boolean) (SweepResult :type Hit%20Result%20Structure%20%28by%20ref%29))
  (bind _asbp_first_person (Utilities|Casting|CastToBP_FirstPerson (Game|GetPlayerCharacter 0)))
  (if (>= (Variables|/Game/MiniGame/Charactere/BP_FirstPerson.BP_FirstPerson_C|GetPlushCollected _asbp_first_person) (Variables|/Game/MiniGame/Charactere/BP_FirstPerson.BP_FirstPerson_C|GetTotalPlush _asbp_first_person))
    (bind _returnvalue (UserInterface|CreateWidget "/Game/Widget/WBP_Victory.WBP_Victory_C"))
    (UserInterface|Viewport|AddtoViewport _returnvalue 0)
    (Utilities|FlowControl|Delay 3.0)
    (Game|OpenLevel(byName) (Variables|Default|GetM_LoopHero))))

(event EventBeginPlay)

(event Collision|EventActorBeginOverlap
  (params (OtherActor :type Actor%20Object%20Reference)))

(event EventTick
  (params (DeltaSeconds :type Float%20%28single-precision%29)))

(fn ConstructionScript)